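; JumpComponentBP is a component that makes its owning static mesh actor hop periodically.
; On begin play it copies the player PhysicsBallBP's jump impulse and overrides the mesh's mass to match the ball's.
; A looping timer then calls Jump, which applies an upward impulse to the mesh whenever the player ball is not tethered.
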(event EventBeginPlay
  (bind _asstatic_mesh_actor (Utilities|Casting|CastToStaticMeshActor (Components|GetOwner)))
  (Variables|Default|SetParentMesh _asstatic_mesh_actor)
  (bind _asphysics_ball_bp (Utilities|Casting|CastToPhysicsBallBP (Game|Player|GetPlayerPawn 0)))
  (Variables|Default|Setplayer _asphysics_ball_bp)
  (Variables|Default|SetJumpImpulse (Variables|/Game/RollingBP/Blueprints/PhysicsBallBP.PhysicsBallBP_C|GetJumpImpulse _asphysics_ball_bp))
  (Class|PrimitiveComponent|SetMassOverrideinKg (Variables|/Script/Engine.StaticMeshActor|GetStaticMeshComponent (Variables|Default|GetParentMesh)) "None" (Physics|GetMass (Variables|/Game/RollingBP/Blueprints/PhysicsBallBP.PhysicsBallBP_C|GetBall _asphysics_ball_bp)) true)
  (Utilities|Time|SetTimerbyFunctionName 0 "Jump" (Variables|Default|GetJumpInterval) true))

(event EventTick
  (params (DeltaSeconds :type Float%20%28single-precision%29)))

(fn Jump
  (if (not (Variables|/Game/RollingBP/Blueprints/PhysicsBallBP.PhysicsBallBP_C|GetIsTethered (Variables|Default|Getplayer)))
    (Physics|AddImpulse (Variables|/Script/Engine.StaticMeshActor|GetStaticMeshComponent (Variables|Default|GetParentMesh)) (Math|Vector|MakeVector 0.0 0.0 (Variables|Default|GetJumpImpulse)) "None" false)))