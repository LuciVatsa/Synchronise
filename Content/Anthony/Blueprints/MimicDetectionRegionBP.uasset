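; Trigger region that detects when the player's PhysicsBallBP mimics the movement of LeaderObject.
; While the ball overlaps, a looping timer compares both actors' displacement from recorded start positions, within a spatial tolerance.
; A limited number of consecutive misses is tolerated before the baseline resets.
; Reaching TargetTime calls a named function on TargetObject via a near-zero timer and can tether the ball to the leader, which blocks retriggering.
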(event EventBeginPlay)

(event Collision|EventActorBeginOverlap
  (params (OtherActor :type Actor%20Object%20Reference))
  (bind _asphysics_ball_bp (Utilities|Casting|CastToPhysicsBallBP OtherActor))
  (Variables|Default|SetPlayerCharacter _asphysics_ball_bp)
  (bind _returnvalue (Utilities|Time|SetTimerbyFunctionName 0 "CheckMimicking" (Variables|Default|GetCheckInterval) true)))

(event EventTick
  (params (DeltaSeconds :type Float%20%28single-precision%29)))

(event Collision|EventActorEndOverlap
  (params (OtherActor :type Actor%20Object%20Reference))
  (Utilities|Casting|CastToPhysicsBallBP OtherActor)
  (Utilities|Time|ClearandInvalidateTimerbyHandle (stale Collision|EventActorBeginOverlap _returnvalue)))

(fn ConstructionScript)

(fn CheckMimicking
  (if (<= (Variables|Default|GetTimeMimicked) 0.0)
    (Variables|Default|SetPlayerStartPos (Transformation|GetActorLocation (Variables|Default|GetPlayerCharacter)))
    (Variables|Default|SetLeaderStartPos (Transformation|GetActorLocation (Variables|Default|GetLeaderObject)))
    (Variables|Default|SetTimeMimicked (Variables|Default|GetCheckInterval))
    (Development|PrintString "Not mimicking...")
    (elif (Math|Vector|Equal(Vector) (- (Transformation|GetActorLocation (Variables|Default|GetLeaderObject)) (Variables|Default|GetLeaderStartPos)) (- (Transformation|GetActorLocation (Variables|Default|GetPlayerCharacter)) (Variables|Default|GetPlayerStartPos)) (Variables|Default|GetSpatialTolerance))
      (Variables|Default|SetChecksMissed 0)
      (bind _output_get (Variables|Default|SetTimeMimicked (+ (Variables|Default|GetTimeMimicked) (Variables|Default|GetCheckInterval)) :!label _label))
      (if (and (>= _output_get (Variables|Default|GetTargetTime)) (not (Variables|Default|GetAlreadyTriggered)))
        (Utilities|Time|SetTimerbyFunctionName (Variables|Default|GetTargetObject) (Variables|Default|GetTargetFunction) 1e-06)
        (if (Variables|Default|GetTethers)
          (bind _asphysics_ball_bp (Utilities|Casting|CastToPhysicsBallBP (Variables|Default|GetPlayerCharacter)))
          (Variables|/Game/RollingBP/Blueprints/PhysicsBallBP.PhysicsBallBP_C|SetIsTethered _asphysics_ball_bp true)
          (Variables|/Game/RollingBP/Blueprints/PhysicsBallBP.PhysicsBallBP_C|SetTetheredObject _asphysics_ball_bp (Variables|Default|GetLeaderObject))
          (Variables|Default|SetAlreadyTriggered true)))
      (Development|PrintString "Mimicking!")
      (else
        (bind _result (Math|Integer|IncrementInt (Variables|Default|GetChecksMissed))
          (:%20%20
            (if (> _result (Variables|Default|GetTemporalTolerance))
              (Variables|Default|SetTimeMimicked 0.0)
              (CallFunction|CheckMimicking)
              (else
                (goto _label)))))))))