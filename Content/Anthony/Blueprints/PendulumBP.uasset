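; Pendulum actor that swings back and forth by rotating itself, carrying an attached Ball actor with it.
; On BeginPlay it attaches the Ball with world transforms kept and sets the timeline play rate from PlaySpeed.
; The timeline lerps the actor between Rotation and its negation, restarting from the start whenever it finishes.
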(event EventBeginPlay
  (Transformation|AttachActorToActor (Variables|Default|GetBall) self "None" "KeepWorld" "KeepWorld" "KeepWorld" true)
  (Components|Timeline|SetPlayRate (Variables|Default|GetTimeline_0) (Variables|Default|GetPlaySpeed))
  (bind _newtrack_0 (Timeline|Timeline_0 Play)
    (:Update
      (Transformation|SetActorRotation (Math|Rotator|Lerp(Rotator) (Variables|Default|GetRotation) (* (Variables|Default|GetRotation) -1) _newtrack_0)))
    (:Finished
      (Timeline|Timeline_0 PlayFromStart))))

(event Collision|EventActorBeginOverlap
  (params (OtherActor :type Actor%20Object%20Reference)))

(event EventTick
  (params (DeltaSeconds :type Float%20%28single-precision%29)))

(fn ConstructionScript)