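; SimpleDoorBP is a door actor that slides from its starting position by a CloseOffset vector when opened.
; BeginPlay stores the start location, and the Open function calls OpenEvent, which plays a timeline that lerps the actor to the offset position.
; Movement is unswept, and the file contains no closing logic.
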(event Custom|OpenEvent
  (bind _newtrack_0 (Timeline|OpenTimeline Play)
    (:Update
      (Transformation|SetActorLocation (Math|Vector|Lerp(Vector) (Variables|Default|GetStartPos) (+ (Variables|Default|GetStartPos) (Variables|Default|GetCloseOffset)) _newtrack_0) false false))))

(event EventBeginPlay
  (Variables|Default|SetStartPos (Transformation|GetActorLocation)))

(event Collision|EventActorBeginOverlap
  (params (OtherActor :type Actor%20Object%20Reference)))

(event EventTick
  (params (DeltaSeconds :type Float%20%28single-precision%29)))

(fn ConstructionScript)

(fn Open
  (CallFunction|OpenEvent))