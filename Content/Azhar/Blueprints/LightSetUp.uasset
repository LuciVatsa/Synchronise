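; LightSetUp is a puzzle light actor that a PhysicsBallBP switches on by overlapping its Box.
; It toggles the PointLight's visibility, sets LightOn, then reverses both after a delay; TurnLightOn and TurnLightOff events enter the same logic.
; CheckLightOn recursively ANDs the state along a chain of LightObj references.
; The instance flagged First polls the chain every Tick and prints "Level cleared!" while all are lit.
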(event OnComponentBeginOverlap(Box)
  (params (OverlappedComponent :type Primitive%20Component%20Object%20Reference) (OtherActor :type Actor%20Object%20Reference) (OtherComp :type Primitive%20Component%20Object%20Reference) (OtherBodyIndex :type Integer) (bFromSweep :type Boolean) (SweepResult :type Hit%20Result%20Structure%20%28by%20ref%29))
  (Utilities|Casting|CastToPhysicsBallBP OtherActor)
  (if (not (Variables|Default|GetlightOn))
    (Rendering|ToggleVisibility (Variables|Default|GetPointLight) false)
    (Variables|Default|SetlightOn true)
    (Utilities|FlowControl|Sequence
      (:then_0
        (Utilities|FlowControl|Delay 2e+01)
        (Rendering|ToggleVisibility (Variables|Default|GetPointLight) false)
        (Variables|Default|SetlightOn false)))))

(event Custom|TurnLightOn
  (if (not (Variables|Default|GetlightOn))
    (Rendering|ToggleVisibility (Variables|Default|GetPointLight) false)
    (Variables|Default|SetlightOn true)
    (Utilities|FlowControl|Sequence
      (:then_0
        (Utilities|FlowControl|Delay 2e+01)
        (Rendering|ToggleVisibility (Variables|Default|GetPointLight) false)
        (Variables|Default|SetlightOn false)))))

(event Custom|TurnLightOff
  (Rendering|ToggleVisibility (Variables|Default|GetPointLight) false)
  (Variables|Default|SetlightOn false))

(event EventBeginPlay)

(event Collision|EventActorBeginOverlap
  (params (OtherActor :type Actor%20Object%20Reference)))

(event EventTick
  (params (DeltaSeconds :type Float%20%28single-precision%29))
  (if (Variables|Default|GetFirst)
    (bind _lightison (CallFunction|CheckLighton))
    (if _lightison
      (Development|PrintString "Level cleared!"))))

(fn ConstructionScript)

(fn CheckLighton
  (LocalVariables|SetResult (Variables|Default|GetlightOn))
  (if (Utilities|IsValid (Variables|Default|GetlightObj))
    (bind _lightison (CallFunction|CheckLighton (Variables|Default|GetlightObj)))
    (LocalVariables|SetResult (and _lightison (LocalVariables|GetResult))))
  (return (LocalVariables|GetResult)))