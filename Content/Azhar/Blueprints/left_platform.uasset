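; Platform that lowers its static mesh and lights up when a PhysicsBallBP enters its trigger box.
; A timeline drives a vertical lerp of the mesh's relative location between two fixed points.
; Any actor leaving the box reverses the timeline after a short delay, and the light turns off once the mesh is back at the top.
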(event OnComponentBeginOverlap(Box)
  (params (OverlappedComponent :type Primitive%20Component%20Object%20Reference) (OtherActor :type Actor%20Object%20Reference) (OtherComp :type Primitive%20Component%20Object%20Reference) (OtherBodyIndex :type Integer) (bFromSweep :type Boolean) (SweepResult :type Hit%20Result%20Structure%20%28by%20ref%29))
  (Utilities|Casting|CastToPhysicsBallBP OtherActor)
  (Default|TurnLighton (Variables|Default|Getlight))
  (bind (_direction _newtrack_0) (Timeline|Timeline_0 Play)
    (:Update
      (Transformation|SetRelativeLocation (Variables|Default|GetStaticMeshComponent0) (Math|Vector|Lerp(Vector) "-0.399957,0.000000,-21.749878" "-0.399957,0.000000,-173.749878" _newtrack_0) false false))
    (:Finished
      (switch Utilities|FlowControl|Switch|SwitchonETimelineDirection _direction
        (:Backward
          (Default|TurnLightOff (Variables|Default|Getlight)))))))

(event OnComponentEndOverlap(Box)
  (params (OverlappedComponent :type Primitive%20Component%20Object%20Reference) (OtherActor :type Actor%20Object%20Reference) (OtherComp :type Primitive%20Component%20Object%20Reference) (OtherBodyIndex :type Integer))
  (Utilities|FlowControl|Delay 3.0)
  (bind (_direction _newtrack_0) (Timeline|Timeline_0 Reverse)
    (:Update
      (Transformation|SetRelativeLocation (Variables|Default|GetStaticMeshComponent0) (Math|Vector|Lerp(Vector) "-0.399957,0.000000,-21.749878" "-0.399957,0.000000,-173.749878" _newtrack_0) false false))
    (:Finished
      (switch Utilities|FlowControl|Switch|SwitchonETimelineDirection _direction
        (:Backward
          (Default|TurnLightOff (Variables|Default|Getlight)))))))

(event EventTick
  (params (DeltaSeconds :type Float%20%28single-precision%29)))

(fn ConstructionScript)