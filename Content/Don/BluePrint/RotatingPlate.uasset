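; RotatingPlate is an actor Blueprint that periodically drops DroppingBallPawn instances from above.
; Tick accumulates a cooldown and, once it reaches two seconds, resets it and spawns the pawn through SpawnAIFromClass.
; The spawn point sits high above the plate, offset horizontally using sine and cosine of an angle derived from its current rotation.
; The graph itself applies no rotation.
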(event EventTick
  (params (DeltaSeconds :type Float%20%28single-precision%29))
  (bind _returnvalue (Transformation|GetActorRotation))
  (bind _returnvalue_2 (Math|Rotator|GetRotationXVector _returnvalue))
  (bind _returnvalue_3 (Class|KismetMathLibrary|ToQuaterion(Vector) _returnvalue_2))
  (bind _returnvalue_4 (Class|KismetMathLibrary|QuatEuler _returnvalue_3))
  (bind _z (Math|Vector|BreakVector _returnvalue_4))
  (Math|Float|CompareFloat (Variables|Default|GetCoolDown) 2.0
    (:>
      (Variables|Default|SetCoolDown 0.0 :!label _label)
      (AI|SpawnAIFromClass "/Game/Don/BluePrint/DroppingBallPawn.DroppingBallPawn_C" 0 (+ (Transformation|GetActorLocation) (Math|Vector|MakeVector (* 1.9e+02 (Math|Trig|Cos(Degrees) _z)) (* 1.9e+02 (Math|Trig|Sin(Degrees) _z)) 2e+03)) _returnvalue false))
    (:==
      (goto _label))
    (:<
      (Variables|Default|SetCoolDown (+ DeltaSeconds (Variables|Default|GetCoolDown))))))

(fn ConstructionScript)